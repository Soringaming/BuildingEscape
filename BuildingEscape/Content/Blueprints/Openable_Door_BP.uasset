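; Door actor that swings open and closed in response to open and close events from its OpenDoor member.
; It stores its starting rotation on BeginPlay, then plays or reverses the DoorSwing timeline, applying the timeline's yaw relative to that rotation.
; A sound event track on the timeline triggers the door sound at the actor's location.
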(event `self.ReceiveBeginPlay`
  (set `self.Initial Rotation ` (`self.K2_GetActorRotation`)))

(event `self.OpenDoor.OnOpen`
  (bind (_direction _open_angle) (`Timeline|Door Swing` :!label _label)
    (:`Update`
      (`self.K2_SetActorRotation` (`KismetMathLibrary.ComposeRotators` (`KismetMathLibrary.MakeRotator` 0.0 0.0 _open_angle) (`self.Initial Rotation `))))
    (:`Sound Timing`
      (`GameplayStatics.PlaySoundAtLocation` "/Game/Audio/OpenDoor2-2.OpenDoor2-2" (`self.K2_GetActorLocation`)))))

(event `self.OpenDoor.OnClose`
  (goto _label :!via `Reverse`))

(fn `UserConstructionScript`)